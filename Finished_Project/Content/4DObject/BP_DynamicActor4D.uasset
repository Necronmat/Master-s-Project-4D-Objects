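; Generated dynamic mesh actor that displays a 4D shape and slowly spins around its yaw axis every tick.
; On mesh rebuild it switches on the shape type to one of the regular polytope builders (5 to 600-cell) or a random or custom point-based one.
; Each builder receives the object's W transform and limits plus the current W position and angle, and its result is set on the dynamic mesh component.
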(event EventBeginPlay)

(event Collision|EventActorBeginOverlap
  (params (OtherActor :type Actor%20Object%20Reference)))

(event EventTick
  (params (DeltaSeconds :type Float%20%28single-precision%29))
  (Transformation|AddActorLocalRotation (Math|Rotator|MakeRotator 0.0 0.0 0.1) false false))

(event Events|EventOnRebuildGeneratedMesh
  (params (TargetMesh :type Dynamic%20Mesh%20Object%20Reference))
  (bind _mpoints4d (Variables|Default|GetmPoints4D))
  (bind _manglew (Variables|Default|GetmAngleW))
  (bind _mminw (Variables|Default|GetmMinW))
  (bind _mcurrentw (Variables|Default|GetmCurrentW))
  (bind _mmaxw (Variables|Default|GetmMaxW))
  (bind _mcurrentanglew (Variables|Default|GetmCurrentAngleW))
  (bind _mpositionw (Variables|Default|GetmPositionW))
  (bind _mscalew (Variables|Default|GetmScaleW))
  (switch Utilities|FlowControl|Switch|SwitchonE4DShape (Variables|Default|GetmShapeType)
    (:Cell5
      (bind _returnvalue (Class|DynamicActor4D|Append5Cell TargetMesh _mcurrentanglew _mcurrentw _mpositionw _mscalew _manglew _mmaxw _mminw))
      (Class|DynamicMeshComponent|SetDynamicMesh (Variables|Default|GetDynamicMeshComponent) _returnvalue))
    (:Cell8
      (bind _returnvalue_2 (Class|DynamicActor4D|Append8Cell TargetMesh _mcurrentanglew _mcurrentw _mpositionw _mscalew _manglew _mmaxw _mminw))
      (Class|DynamicMeshComponent|SetDynamicMesh (Variables|Default|GetDynamicMeshComponent) _returnvalue_2))
    (:Cell16
      (bind _returnvalue_3 (Class|DynamicActor4D|Append16Cell TargetMesh _mcurrentanglew _mcurrentw _mpositionw _mscalew _manglew _mmaxw _mminw))
      (Class|DynamicMeshComponent|SetDynamicMesh (Variables|Default|GetDynamicMeshComponent) _returnvalue_3))
    (:Cell24
      (bind _returnvalue_4 (Class|DynamicActor4D|Append24Cell TargetMesh _mcurrentanglew _mcurrentw _mpositionw _mscalew _manglew _mmaxw _mminw))
      (Class|DynamicMeshComponent|SetDynamicMesh (Variables|Default|GetDynamicMeshComponent) _returnvalue_4))
    (:Cell120
      (bind _returnvalue_5 (Class|DynamicActor4D|Append120Cell TargetMesh _mcurrentanglew _mcurrentw _mpositionw _mscalew _manglew _mmaxw _mminw))
      (Class|DynamicMeshComponent|SetDynamicMesh (Variables|Default|GetDynamicMeshComponent) _returnvalue_5))
    (:Cell600
      (bind _returnvalue_6 (Class|DynamicActor4D|Append600Cell TargetMesh _mcurrentanglew _mcurrentw _mpositionw _mscalew _manglew _mmaxw _mminw))
      (Class|DynamicMeshComponent|SetDynamicMesh (Variables|Default|GetDynamicMeshComponent) _returnvalue_6))
    (:Random
      (bind _returnvalue_7 (Class|DynamicActor4D|AppendRandom4D TargetMesh _mcurrentanglew _mcurrentw _mpositionw _mscalew _manglew _mmaxw _mminw _mpoints4d))
      (Class|DynamicMeshComponent|SetDynamicMesh (Variables|Default|GetDynamicMeshComponent) _returnvalue_7))
    (:Custom
      (bind _returnvalue_8 (Class|DynamicActor4D|AppendCustom4D TargetMesh _mcurrentanglew _mcurrentw _mpositionw _mscalew _manglew _mmaxw _mminw _mpoints4d))
      (Class|DynamicMeshComponent|SetDynamicMesh (Variables|Default|GetDynamicMeshComponent) _returnvalue_8))))

(fn ConstructionScript)